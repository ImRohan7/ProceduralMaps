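; BP_Room is a cube-mesh room actor that nudges other overlapping rooms away along world Y.
; BeginPlay assigns the cube static mesh.
; Each Tick, it finds BP_Room actors overlapping that mesh and offsets each by a small random, non-negative Y step without sweeping, a brute-force way to spread overlapping rooms.
; The physics-simulation call is unconnected and never runs.
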(event EventBeginPlay
  (Components|StaticMesh|SetStaticMesh (Variables|Default|GetMeshCube) "/Game/Geometry/Meshes/1M_Cube.1M_Cube"))

(event Collision|EventActorBeginOverlap
  (params (OtherActor :type Actor%20Object%20Reference)))

(event EventTick
  (params (DeltaSeconds :type Float%20%28single-precision%29))
  (for _array_element (Collision|GetOverlappingActors (Variables|Default|GetMeshCube) "BP_Room_C" :!class /Script/Engine.PrimitiveComponent)
    (Transformation|AddActorWorldOffset _array_element (Math|Vector|MakeVector 0.0 (Math|Conversions|ToFloat(Integer) (Math|Random|RandomInteger 7)) 0.0))))

(fn ConstructionScript)